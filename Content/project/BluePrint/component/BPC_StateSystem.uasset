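; BPC_StateSystem is a state component that tracks health, stamina and sharpness, setting each current value to its maximum on BeginPlay.
; Increase and decrease functions adjust these values and return status flags for success, full or depleted, though IncreaseSharpness adds to MaxSharpness and compares against MaxStamina.
; DecreaseHealth takes a damage struct, skips damage when ignoring or dead, sets death at zero, and returns a damage response for interruptible or lethal hits.
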(event `self.ReceiveBeginPlay`
  (`self.SetCurrent_value`))

(fn `Decrease_health`
  (params (Damage_type :type "/Game/project/BluePrint/Struct/ST_Damege_Info Structure"))
  (returns (`is Dead` :type Boolean) (Is_demaged :type Boolean) (Damage_response :type "/Game/project/BluePrint/enum/BPE_Damege_Responed Enum"))
  (bind (_amount _damame_type _demage_responed _take_damaged _ignore_damage _should_interuptible) (break `/Game/project/BluePrint/Struct/ST_Damege_Info` Damage_type))
  ;[1 1 1] 코멘트
  (if (and (not (`self.Isignore`)) (not (`self.isDead`)))
    (bind _output_get (set `self.Current_HP` (- (`self.Current_HP`) _amount)))
    (`KismetSystemLibrary.PrintString` (`KismetStringLibrary.Conv_DoubleToString` _output_get))
    (if (> _output_get 0.0)
      (if _should_interuptible
        (return (stale _output_get_2) true _demage_responed))
      (else
        (set `self.Current_HP` 0.0)
        (bind _output_get_2 (set `self.isDead` true))
        (return _output_get_2 true _demage_responed)))
    (elif _ignore_damage
      (return false false "NewEnumerator0"))))

(fn `Decrease_Sharpness`
  (params (B :type "Float (double-precision)"))
  (returns (`Current Sharpness` :type "Float (double-precision)") (`no Sharpness` :type Boolean))
  (bind _returnvalue (- (`self.Current_Sharpness`) B))
  (if (> _returnvalue 0.0)
    (bind _output_get (set `self.Current_Sharpness` _returnvalue))
    (return _output_get false)
    (else
      (bind _output_get_2 (set `self.Current_Sharpness` 0.0))
      (bind _output_get_3 (set `self.isNoSharpness` true))
      (return _output_get_2 _output_get_3))))

(fn `Decrease_stamina`
  (params (Decrease_point :type "Float (double-precision)"))
  (returns (`Decrease stamina` :type "Float (double-precision)") (isNoStamina :type Boolean))
  (bind _returnvalue (- (`self.Current_Stamina`) Decrease_point))
  (if (>= _returnvalue 0.0)
    (bind _output_get (set `self.Current_Stamina` _returnvalue))
    (return _output_get false)
    (else
      (bind _output_get_2 (set `self.Current_Stamina` 0.0))
      (bind _output_get_3 (set `self.IsNoStamina` true))
      (return _output_get_2 _output_get_3))))

(fn `Increase_health`
  (params (heal_HP :type "Float (double-precision)"))
  (returns (`Increase health` :type "Float (double-precision)") (Success :type Boolean))
  (if (not (`self.isDead`))
    (set `self.Current_HP` (`KismetMathLibrary.FClamp` (+ heal_HP (`self.Current_HP`)) 0.0 (`self.Max_HP`)))
    (return 0.0 true)))

(fn `Increase_Sharpness`
  (params (B :type "Float (double-precision)"))
  (returns (`current Sharpness` :type "Float (double-precision)") (isMax :type Boolean))
  (bind _returnvalue (+ B (`self.Max_Sharpness`)))
  (if (> _returnvalue (`self.Max_Stamina`))
    (bind _output_get (set `self.Current_Sharpness` (`self.Max_Sharpness`)))
    (return _output_get true)
    (else
      (bind _output_get_2 (set `self.Current_Sharpness` _returnvalue))
      (return _output_get_2 false))))

(fn `Increase_stamina`
  (params (Heal_Stamina :type "Float (double-precision)"))
  (returns (`Increase Health` :type "Float (double-precision)") (`is max` :type Boolean))
  (bind _returnvalue (+ Heal_Stamina (`self.Current_Stamina`)))
  (bind _output_get (set `self.Current_Stamina` _returnvalue))
  (if (> _output_get (`self.Max_Stamina`))
    (bind _output_get_2 (set `self.Current_Stamina` (`self.Max_Stamina`)))
    (return _output_get_2 true)
    (else
      (return _returnvalue false))))

(fn `SetCurrent_value`
  (set `self.Current_HP` (`self.Max_HP`))
  (set `self.Current_Stamina` (`self.Max_Stamina`))
  (set `self.Current_Sharpness` (`self.Max_Sharpness`)))