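; Player combat component for BP_player, driving a transforming sword-and-shield/axe weapon with draw, combos, charged attacks, bottle charging and upgrades.
; Input events select attack montages by mode and combo index, with synchronized weapon montages.
; Montage notifies release the IsPlaying lock, advance MultiGate combos, reattach the shield between bone sockets, and update bottle charges or upgrade windows.
; A looping timer resets combo counters, and an attack-type enum selects damage values.
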(event `play_wp_montage`
  ;[1 1 1] 무기 애니메이션 재생
  (`|PlayMontage` (`self.Battle_shild_mesh`) (`|GetArrayItem` (`self.M_Anim_shild`) (`self.Shild_Anim_index`))
    (:`then`
      (`|PlayMontage` (`self.Battle_sward_mesh`) (`|GetArrayItem` (`self.M_Anim_sward`) (`self.Sward_Anim_index`)) :!label _label))))

(event `Play_only_sward_montage`
  ;[1 1 1] 무기 애니메이션 재생
  (goto _label))

(event `self.ReceiveBeginPlay`
  ;[1 1 1] 시작 컴포넌트 설정
  (bind _asbp_player (cast `/Game/project/BluePrint/Pl/BP_player` (`self.GetOwner`)))
  (bind _output_get (set `self.player_character` _asbp_player))
  (set `self.character_mesh` (`Character.Mesh` _output_get))
  (set `self.Battle_shild_mesh` (`/Game/project/BluePrint/Pl/BP_player.battle_shild` _asbp_player))
  (set `self.Battle_sward_mesh` (`/Game/project/BluePrint/Pl/BP_player.battle_sward` _asbp_player)))

(event `Reset_counter`
  ;[1 1 1] 콤보 카운트 초기화
  (`KismetSystemLibrary.K2_SetTimerDelegate` (delegate `reset`) 1.5 true))

(event `reset`
  ;[1 1 1] 콤보 카운트 초기화
  (set `self.combo_count_sward` 0)
  (set `self.combo_count_axe_L` 0)
  (set `self.combo_count_axe_R` 0)
  (set `self.combo_count_sward_LR` 0)
  (`KismetSystemLibrary.PrintString` "reset count"))

(event `EnhancedInput|/Game/ThirdPerson/Input/Actions/IA_Attack`
  (params (ActionValue :type Boolean) (ElapsedSeconds :type "Float (double-precision)") (TriggeredSeconds :type "Float (double-precision)") (InputAction :type "InputAction Object Reference" :default "/Game/ThirdPerson/Input/Actions/IA_Attack.IA_Attack"))
  (bind _player_character (`self.player_character`))
  (bind _player_character_2 (`self.player_character`))
  (bind _character_mesh (`self.character_mesh`))
  ;[1 1 1] 공격 - 좌클릭
  (:`Started`
    (set `self.Attack_Damage_type` "NewEnumerator2")
    (`self.Attack_Type_Damage`)
    (if (`/Game/project/BluePrint/Pl/BP_player.isPlaying` (`self.player_character`))
      _
      (elif (and (not (`self.is_attack`)) (`/Game/project/BluePrint/Pl/BP_player.is Battle_start` (`self.player_character`)))
        (if (`/Game/project/BluePrint/Pl/BP_player.is_mode_axe` (`self.player_character`))
          ;;[1 1 1] 도끼 - 일반공격
          (set `self.is_attack` true)
          (`|PlayMontage` (`self.character_mesh`) (`|GetArrayItem` (`self.M_Attack_Axe_L`) (`self.combo_count_axe_L`))
            (:`then`
              (`self.isplaying` :!label _label
                (:`then2`
                  (`|MultiGate` false true
                    (:`Out 0`
                      (`self.combo_axe_L` 1))
                    (:`Out 1`
                      (`self.combo_axe_L` 0)))
                  (`self.Reset_counter`))))
            (:`OnNotifyBegin`
              (goto _label :!via `is_playing_false`)))
          (elif (`PlayerController.IsInputKeyDown` (`GameplayStatics.GetPlayerController` 0) "Q")
            ;;[1 1 1] 검방 상태에서 도끼로 변환
            (`|PlayMontage` (`self.character_mesh`) "/Game/project/BluePrint/montage/player/Q_change_axe.Q_change_axe"
              (:`then`
                (`self.isplaying` :!label _label_2
                  (:`then`
                    (`/Game/project/BluePrint/Pl/BP_player.set_Axe_speed` _player_character_2)
                    (set `/Game/project/BluePrint/Pl/BP_player.is_mode_axe` true _player_character_2))))
              (:`OnCompleted`
                (goto _label_2 :!via `is_playing_false`))
              (:`OnNotifyBegin`
                (`self.Sld_change_bone_shild_to_sward`)
                (set `self.Sward_Anim_index` 4)
                (set `self.Shild_Anim_index` 6)
                (`self.play_wp_montage`)))
            (else
              ;;[1 1 1] 검방 - 일반공격
              (set `self.is_attack` true)
              (`|PlayMontage` (`self.character_mesh`) (`|GetArrayItem` (`self.M_Attack_sward_L`) (`self.combo_count_sward`))
                (:`then`
                  (`self.isplaying` :!label _label_3
                    (:`then2`
                      (`|MultiGate` false true
                        (:`Out 0`
                          (`self.combo_sward_L` 1))
                        (:`Out 1`
                          (`self.combo_sward_L` 2))
                        (:`Out 2`
                          (`self.combo_sward_L` 0)))
                      (`self.Reset_counter`))))
                (:`OnNotifyBegin`
                  (goto _label_3 :!via `is_playing_false`))))))
        (else
          ;;[1 1 1] 발도
          (if (`/Game/project/BluePrint/Pl/BP_player.is move` (`self.player_character`))
            (`|PlayMontage` _character_mesh "/Game/project/BluePrint/montage/player/battle_start_moveAttack.battle_start_moveAttack"
              (:`then`
                (set `self.Sward_Anim_index` 1)
                (`self.Play_only_sward_montage`))
              (:`OnCompleted`
                (goto _label_4 :!via `is_playing_false`)))
            (else
              (`|PlayMontage` _character_mesh "/Game/project/BluePrint/montage/player/Battle_start.Battle_start"
                (:`then`
                  (set `self.Sward_Anim_index` 1)
                  (set `self.Shild_Anim_index` 10)
                  (`self.play_wp_montage`))
                (:`OnCompleted`
                  (goto _label_4 :!via `is_playing_false`)))))
          (`self.isplaying` :!label _label_4
            (:`then2`
              (set `/Game/project/BluePrint/Pl/BP_player.is Battle_start` true _player_character)
              (`/Game/project/BluePrint/Pl/BP_player.set _battle_speed` _player_character))))))))

(event `EnhancedInput|/Game/ThirdPerson/Input/Actions/IA_Attack`
  (params (ActionValue :type Boolean) (ElapsedSeconds :type "Float (double-precision)") (TriggeredSeconds :type "Float (double-precision)") (InputAction :type "InputAction Object Reference" :default "/Game/ThirdPerson/Input/Actions/IA_Attack.IA_Attack"))
  ;[1 1 1] 공격 - 좌클릭
  ;;[1 1 1] 코멘트
  (:`Started`
    (if (`/Game/project/BluePrint/Pl/BP_player.isPlaying` (`self.player_character`))
      _
      (elif (`self.Multi_input_mouse`)
        _))))

(event `EnhancedInput|/Game/ThirdPerson/Input/Actions/IA_ATTack_R`
  (params (ActionValue :type Boolean) (ElapsedSeconds :type "Float (double-precision)") (TriggeredSeconds :type "Float (double-precision)") (InputAction :type "InputAction Object Reference" :default "/Game/ThirdPerson/Input/Actions/IA_ATTack_R.IA_ATTack_R"))
  ;[1 1 1] 공격 - 우클릭
  ;;[1 1 1] 코멘트
  (:`Started`
    (if (`/Game/project/BluePrint/Pl/BP_player.isPlaying` (`self.player_character`))
      _
      (elif (`self.Multi_input_mouse`)
        _))))

(event `EnhancedInput|/Game/ThirdPerson/Input/Actions/IA_ATTack_R`
  (params (ActionValue :type Boolean) (ElapsedSeconds :type "Float (double-precision)") (TriggeredSeconds :type "Float (double-precision)") (InputAction :type "InputAction Object Reference" :default "/Game/ThirdPerson/Input/Actions/IA_ATTack_R.IA_ATTack_R"))
  (bind _player_character (`self.player_character`))
  (bind _character_mesh (`self.character_mesh`))
  (bind _character_mesh_2 (`self.character_mesh`))
  (bind _player_character_2 (`self.player_character`))
  (bind _player_character_3 (`self.player_character`))
  (bind _bottle_charge_stack (`/Game/project/BluePrint/Pl/BP_player.Bottle_Charge Stack` _player_character))
  (:`Started`
    ;[1 1 1] 공격 - 우클릭
    (set `self.Attack_Damage_type` "NewEnumerator2")
    (`self.Attack_Type_Damage`)
    (if (`/Game/project/BluePrint/Pl/BP_player.isPlaying` (`self.player_character`))
      _
      (elif (`/Game/project/BluePrint/Pl/BP_player.is Battle_start` _player_character_2)
        (if (`/Game/project/BluePrint/Pl/BP_player.is_mode_axe` _player_character_2)
          ;;[1 1 1] 도끼 - 특수공격
          (set `self.is_attack` true)
          (`|PlayMontage` (`self.character_mesh`) (`|GetArrayItem` (`self.M_Attack_Axe_R`) (`self.combo_count_axe_R`))
            (:`then`
              (`self.isplaying` :!label _label
                (:`then2`
                  (`|MultiGate` false true
                    (:`Out 0`
                      (`self.combo_axe_R` 1))
                    (:`Out 1`
                      (`self.combo_axe_R` 0)))
                  (`self.Reset_counter`))))
            (:`OnNotifyBegin`
              (goto _label :!via `is_playing_false`)))
          (else
            ;;[1 1 1] 차징
            (if (`PlayerController.IsInputKeyDown` (`GameplayStatics.GetPlayerController` 0) "Q")
              (bind _notifyname (`|PlayMontage` _character_mesh_2 "/Game/project/BluePrint/montage/player/charge_shild.charge_shild")
                (:`then`
                  (`self.isplaying` :!label _label_2
                    (:`then`
                      (set `self.Shild_Anim_index` 13)
                      (set `self.Sward_Anim_index` 9)
                      (`self.play_wp_montage`))))
                (:`OnCompleted`
                  (goto _label_2 :!via `is_playing_false`))
                (:`OnNotifyBegin`
                  (switch `name` _notifyname
                    (:`change_bone_shild`
                      (`self.Sld_change_bone_shild_to_sward`))
                    (:`change_bone_shild_end`
                      (`self.Sld_change_bone_sward_to_shild`))
                    (:`charge_bottle`
                      (`/Game/project/BluePrint/UI/WBP_UHD.Reset_bottle_color` (`/Game/project/BluePrint/UI/UMG_HUD.Player_UI` (`/Game/project/BluePrint/Pl/BP_player.UI` _player_character)) _bottle_charge_stack)
                      (set `/Game/project/BluePrint/Pl/BP_player.Bottle_charge` _bottle_charge_stack (`self.player_character`))
                      (set `/Game/project/BluePrint/Pl/BP_player.Bottle_Charge Stack` 0 _player_character)))))
              (else
                (`|PlayMontage` _character_mesh_2 "/Game/project/BluePrint/montage/player/Attack_R.Attack_R"
                  (:`then`
                    (set `self.is_complete_action` true))))))))))
  (:`Completed`
    (if (`self.is_complete_action`)
      (if (not (`/Game/project/BluePrint/Pl/BP_player.isPlaying` (`self.player_character`)))
        ;;[1 1 1] 검방 - 특수 공격
        (if (and (`/Game/project/BluePrint/Pl/BP_player.is Battle_start` _player_character_3) (not (`/Game/project/BluePrint/Pl/BP_player.is_mode_axe` _player_character_3)))
          (if (>= TriggeredSeconds 0.8)
            (set `self.Attack_Damage_type` "NewEnumerator3")
            (`self.Attack_Type_Damage`)
            (`|PlayMontage` _character_mesh "/Game/project/BluePrint/montage/player/Attack_R2.Attack_R2"
              (:`then`
                (`self.isplaying` :!label _label_3
                  (:`then2`
                    (`self.combo_sward_L` 2)
                    (`self.Reset_counter`))))
              (:`OnCompleted`
                (set `self.is_complete_action` false :!label _label_4))
              (:`OnNotifyBegin`
                (goto _label_3 :!via `is_playing_false`)))
            (else
              (`|PlayMontage` _character_mesh "/Game/project/BluePrint/montage/player/Attack_R3.Attack_R3"
                (:`then`
                  (`self.isplaying` :!label _label_5
                    (:`then2`
                      (goto _label_4))))
                (:`OnCompleted`
                  (goto _label_5 :!via `is_playing_false`))))))))))

(event `Key|F`
  (params (Key :type "Key Structure"))
  (bind _player_character (`self.player_character`))
  (bind _player_ui (`/Game/project/BluePrint/UI/UMG_HUD.Player_UI` (`/Game/project/BluePrint/Pl/BP_player.UI` _player_character)))
  ;[1 1 1] 공격 - 동시 클릭
  (:`Pressed`
    (set `self.Attack_Damage_type` "NewEnumerator3")
    (if (not (`/Game/project/BluePrint/Pl/BP_player.isPlaying` (`self.player_character`)))
      (set `self.is_attack` true)
      (`self.Attack_Type_Damage`)
      (bind _notifyname (`|PlayMontage` (`self.character_mesh`) (`|GetArrayItem` (`self.M_Attack_sward_LR`) (`self.combo_count_sward_LR`)))
        (:`then`
          (`self.isplaying` :!label _label
            (:`then`
              (switch `int` (`self.combo_count_sward_LR`)
                (:`1`
                  (set `self.Shild_Anim_index` 3)
                  (`self.play_wp_montage`))
                (:`2`
                  (set `self.Shild_Anim_index` 4 :!label _label_2)
                  (set `self.Sward_Anim_index` 3))
                (:`3`
                  (goto _label_2))))
            (:`then2`
              (`|MultiGate` false true
                (:`Out 0`
                  (`self.combo_sward_LR` 1))
                (:`Out 1`
                  (if (`self.Upgrade_shild`)
                    (`self.combo_sward_LR` 3)
                    (else
                      (`self.combo_sward_LR` 2))))
                (:`Out 2`
                  (`self.combo_sward_LR` 0)))
              (`self.Reset_counter`))))
        (:`OnNotifyBegin`
          (switch `name` _notifyname
            (:`Default`
              (goto _label :!via `is_playing_false`))
            (:`LR_battle_3`
              (goto _label :!via `is_playing_false`))
            (:`begin_UP_axe`
              (set `self.is_upgrade_axe` true)
              (set `self.is_upgrade_shild` true)
              (`self.isplaying` :!via `is_playing_false`))
            (:`end_UP_axe`
              (set `self.is_upgrade_axe` false)
              (set `self.is_upgrade_shild` false))
            (:`LR_attack_change_bone_shild`
              (`self.Sld_change_bone_shild_to_sward`)
              (`self.play_wp_montage`))
            (:`LR_attack_last_change_bone`
              (`self.Sld_change_bone_sward_to_shild`))
            (:`LR_attack_Last`
              (set `self.Shild_Anim_index` 5)
              (set `self.Sward_Anim_index` 3)
              (`self.play_wp_montage`))
            (:`Delete_bottle_charge`
              (`/Game/project/BluePrint/UI/WBP_UHD.Reset_bottle_color` _player_ui 0)
              (set `/Game/project/BluePrint/Pl/BP_player.Bottle_charge` 0 _player_character))
            (:`Delete_bottle_charge_low`
              (if (> (`/Game/project/BluePrint/Pl/BP_player.Bottle_charge` (`self.player_character`)) 0)
                (`/Game/project/BluePrint/UI/WBP_UHD.Reset_bottle_color` _player_ui 0)
                (`/Engine/EditorBlueprintResources/StandardMacros.DecrementInt` (`/Game/project/BluePrint/Pl/BP_player.Bottle_charge` _player_character))))))))))

(event `EnhancedInput|/Game/ThirdPerson/Input/Actions/IA_Defence`
  (params (ActionValue :type Boolean) (ElapsedSeconds :type "Float (double-precision)") (TriggeredSeconds :type "Float (double-precision)") (InputAction :type "InputAction Object Reference" :default "/Game/ThirdPerson/Input/Actions/IA_Defence.IA_Defence"))
  (bind _player_character (`self.player_character`))
  ;[1 1 1] Q - 방어 or 도끼발도
  (:`Started`
    (set `self.Attack_Damage_type` "NewEnumerator2")
    (if (`/Game/project/BluePrint/Pl/BP_player.isPlaying` (`self.player_character`))
      _
      (elif (`/Game/project/BluePrint/Pl/BP_player.is Battle_start` (`self.player_character`))
        (if (`/Game/project/BluePrint/Pl/BP_player.is_mode_axe` (`self.player_character`))
          (`|ExecutionSequence`
            (:`then_0`
              (`|PlayMontage` (`self.character_mesh`) "/Game/project/BluePrint/montage/player/Q_change_sward_shild.Q_change_sward_shild"
                (:`then`
                  (`self.isplaying` :!label _label))
                (:`OnCompleted`
                  (goto _label :!via `is_playing_false`))
                (:`OnNotifyBegin`
                  (set `/Game/project/BluePrint/Pl/BP_player.is_mode_axe` false (`self.player_character`))
                  (`self.Sld_change_bone_sward_to_shild`)
                  (`/Game/project/BluePrint/Pl/BP_player.set_idle_speed` (`self.player_character`)))))
            (:`then_1`
              (set `self.Sward_Anim_index` 8)
              (set `self.Shild_Anim_index` 12)
              (`self.play_wp_montage`)
              (`KismetSystemLibrary.PrintString` "Q_change_SW")))
          (elif (and (> (`/Game/project/BluePrint/Pl/BP_player.Bottle_charge` (`self.player_character`)) 1) (`self.is_upgrade_shild`))
            (set `self.Upgrade_shild` true)
            (`self.Sld_change_bone_sward_to_shild`)
            (`|ExecutionSequence`
              (:`then_0`
                (`|PlayMontage` (`self.character_mesh`) "/Game/project/BluePrint/montage/player/Q_upgrade_shild.Q_upgrade_shild"
                  (:`then`
                    (`self.isplaying` :!label _label_2
                      (:`then2`
                        (set `self.is_attack` false))))
                  (:`OnCompleted`
                    (`/Game/project/BluePrint/UI/WBP_UHD.Upgrade` (`/Game/project/BluePrint/UI/UMG_HUD.Player_UI` (`/Game/project/BluePrint/Pl/BP_player.UI` (`self.player_character`))))
                    (goto _label_2 :!via `is_playing_false`))))
              (:`then_1`
                (set `self.Sward_Anim_index` 7)
                (set `self.Shild_Anim_index` 11)
                (`self.play_wp_montage`)))))
        (else
          (`self.Sld_change_bone_shild_to_sward`)
          (`|PlayMontage` (`self.character_mesh`) "/Game/project/BluePrint/montage/player/change_axe.change_axe"
            (:`then`
              (`/Game/project/BluePrint/Pl/BP_player.is_axe_activatied` _player_character)
              (`/Game/project/BluePrint/Pl/BP_player.set_Axe_speed` _player_character))
            (:`OnNotifyBegin`
              (set `self.Sward_Anim_index` 5)
              (set `self.Shild_Anim_index` 7)
              (`self.play_wp_montage`)
              (`KismetSystemLibrary.PrintString` "Q_change_axe"))))))))

(event `Key|C`
  (params (Key :type "Key Structure"))
  ;[1 1 1] 도끼 강화
  (:`Pressed`
    (`KismetSystemLibrary.PrintString` "Hello")
    (set `self.Attack_Damage_type` "NewEnumerator3")
    (`self.Attack_Type_Damage`)
    (if (`/Game/project/BluePrint/Pl/BP_player.isPlaying` (`self.player_character`))
      _
      (elif (`self.is_upgrade_axe`)
        (set `self.upgrade_axe` true)
        (set `/Game/project/BluePrint/Pl/BP_player.is_mode_axe` true (`self.player_character`))
        (`|ExecutionSequence`
          (:`then_0`
            (`|PlayMontage` (`self.character_mesh`) "/Game/project/BluePrint/montage/player/C_upgrade_axe.C_upgrade_axe"
              (:`then`
                (`self.isplaying` :!label _label
                  (:`then2`
                    (set `self.is_attack` false)
                    (`/Game/project/BluePrint/Pl/BP_player.set_Axe_speed` (`self.player_character`)))))
              (:`OnCompleted`
                (goto _label :!via `is_playing_false`))
              (:`OnNotifyBegin`
                (`/Game/project/BluePrint/UI/WBP_UHD.Upgrade` (`/Game/project/BluePrint/UI/UMG_HUD.Player_UI` (`/Game/project/BluePrint/Pl/BP_player.UI` (`self.player_character`)))))))
          (:`then_1`
            (`|PlayMontage` (`self.Battle_shild_mesh`) "/Game/project/BluePrint/montage/wp/sh/AM_sld_Upgrade_shild.AM_sld_Upgrade_shild")))))))

(fn `Attack_Type_Damage`
  (returns (Type_damage :type "Float (double-precision)"))
  (bind _output_get (set `self.Attack_type_Damage_` (select `/Game/project/BluePrint/enum/BPE_Damage_Type` (`self.Attack_Damage_type`) :`NewEnumerator1` 200.0 :`NewEnumerator2` 100.0 :`NewEnumerator3` 150.0)))
  (return _output_get))

(fn `combo_axe_L`
  (params (combo_count_axe_L :type Integer))
  (set `self.is_attack` false)
  (set `self.combo_count_axe_L` combo_count_axe_L))

(fn `combo_axe_R`
  (params (combo_count_axe_R :type Integer))
  (set `self.is_attack` false)
  (set `self.combo_count_axe_R` combo_count_axe_R))

(fn `combo_sward_L`
  (params (combo_count_sward :type Integer))
  (set `self.is_attack` false)
  (set `self.combo_count_sward` combo_count_sward))

(fn `combo_sward_LR`
  (params (combo_count_sward_LR :type Integer))
  (set `self.is_attack` false)
  (set `self.combo_count_sward_LR` combo_count_sward_LR))

(fn `Ser_skill_combo_count`
  (params (combo_count_sward :type Integer) (combo_count_sward_LR :type Integer) (combo_count_axe_R :type Integer) (combo_count_axe_L :type Integer)))

(fn `Sld_change_bone_shild_to_sward`
  (`SceneComponent.K2_AttachToComponent` (`self.Battle_shild_mesh`) (`self.character_mesh`) (`/Game/project/BluePrint/Pl/BP_player.Sward_bone` (`self.player_character`)) "KeepRelative" "KeepRelative" "KeepWorld" true)
  (return))

(fn `Sld_change_bone_sward_to_shild`
  (`SceneComponent.K2_AttachToComponent` (`self.Battle_shild_mesh`) (`self.character_mesh`) (`/Game/project/BluePrint/Pl/BP_player.Shild_bone` (`self.player_character`)) "KeepRelative" "KeepRelative" "KeepWorld" true))