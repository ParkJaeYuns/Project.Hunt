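; Animation notify that spawns a ground explosion effect beneath a monster's bone during an animation.
; It acts only when the owner is a bp_monster with ActivatedSlime set, tracing on the Visibility channel from TargetBone down along the mesh's up axis.
; A hit spawns the Niagara explosion at the impact point with a fixed rotation.
; Despite the ANS prefix it fires as a single notify, and it is visual only.
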(fn `Received_Notify`
  (params (MeshComp :type "SkeletalMeshComponent Object Reference") (Animation :type "AnimSequenceBase Object Reference") (EventReference :type "AnimNotifyEventReference Structure (by ref)"))
  (returns (ReturnValue :type Boolean))
  (bind _asbp_monster (cast `/Game/project/BluePrint/Monster/bp_monster` (`ActorComponent.GetOwner` MeshComp)))
  (if (`/Game/project/BluePrint/Monster/bp_monster.Activated_slime` _asbp_monster)
    (bind _mesh (`Character.Mesh` _asbp_monster))
    (bind _returnvalue (`SceneComponent.GetSocketLocation` _mesh (`self.Target_bone`)))
    (bind (_outhit _returnvalue_2) (`KismetSystemLibrary.LineTraceSingle` _returnvalue (+ _returnvalue (* (`SceneComponent.GetUpVector` _mesh) -200.0)) "TraceTypeQuery1"))
    (if _returnvalue_2
      (`NiagaraFunctionLibrary.SpawnSystemAtLocation` "/Game/MsvFx_Niagara_Explosion_Pack_01/Prefabs/Niagara_Explosion_02.Niagara_Explosion_02" (`.ImpactPoint` (`GameplayStatics.BreakHitResult` _outhit)) (struct :`Pitch` 90.0))
      (return true))))

(fn `새 함수`)