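; Anim notify state that turns a monster's attack animation window into a damaging hit against the player.
; Each tick it sphere-traces between the StartBone and EndBone sockets on the monster's mesh and applies that monster's TypeMonsterDamage to any player hit, with no repeat-hit check here.
; On end it fetches the player from the monster's blackboard and clears its IsHitPlayer flag.
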(fn `Received_NotifyEnd`
  (params (MeshComp :type "SkeletalMeshComponent Object Reference") (Animation :type "AnimSequenceBase Object Reference") (EventReference :type "AnimNotifyEventReference Structure (by ref)"))
  (returns (ReturnValue :type Boolean))
  ;[1 1 1] 코멘트
  (bind _asbp_player (cast `/Game/project/BluePrint/Pl/BP_player` (`BlackboardComponent.GetValueAsObject` (`AIBlueprintHelperLibrary.GetBlackboard` (`ActorComponent.GetOwner` MeshComp)) "Player")))
  (set `/Game/project/BluePrint/Pl/BP_player.isHit_player` false _asbp_player)
  (return true))

(fn `Received_NotifyTick`
  (params (MeshComp :type "SkeletalMeshComponent Object Reference") (Animation :type "AnimSequenceBase Object Reference") (FrameDeltaTime :type "Float (single-precision)") (EventReference :type "AnimNotifyEventReference Structure (by ref)"))
  (returns (ReturnValue :type Boolean))
  ;[1 1 1] 코멘트
  (bind _asbp_monster (cast `/Game/project/BluePrint/Monster/bp_monster` (`ActorComponent.GetOwner` MeshComp)))
  (bind _mesh (`Character.Mesh` _asbp_monster))
  (bind _outhit (`KismetSystemLibrary.SphereTraceSingleForObjects` :`WorldContextObject` MeshComp :`Start` (`SceneComponent.GetSocketLocation` _mesh (`self.Start_bone`)) :`End` (`SceneComponent.GetSocketLocation` _mesh (`self.End_bone`)) :`Radius` 100.0 :`ObjectTypes` (`|MakeArray` "ObjectTypeQuery7" :!type "EObjectTypeQuery Enum") :`DrawTime` 2.0))
  (bind (_bblockinghit _binitialoverlap _time _distance _location _impactpoint _normal _impactnormal _physmat _hitactor) (`GameplayStatics.BreakHitResult` _outhit))
  (if _bblockinghit
    (bind _asbp_player (cast `/Game/project/BluePrint/Pl/BP_player` _hitactor))
    (`GameplayStatics.ApplyDamage` _asbp_player (`/Game/project/BluePrint/Monster/bp_monster.Type_monsterDamage` _asbp_monster) null _asbp_monster)
    (return false)))