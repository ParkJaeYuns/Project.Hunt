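; Anim notify state that serves as the damage window for the player's sword attacks against monsters.
; Each tick, it sphere-traces along BattleSward between two bone sockets and applies the attack system's AttackTypeDamage to a hit bp_monster.
; The tick has no repeat-hit guard of its own.
; When the window ends, it clears IsHit on the player's MonsterActor, or prints a debug string if that reference is invalid.
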(fn `Received_NotifyEnd`
  (params (MeshComp :type "SkeletalMeshComponent Object Reference") (Animation :type "AnimSequenceBase Object Reference") (EventReference :type "AnimNotifyEventReference Structure (by ref)"))
  (returns (ReturnValue :type Boolean))
  ;[1 1 1] 코멘트
  (bind _asbp_player (cast `/Game/project/BluePrint/Pl/BP_player` (`ActorComponent.GetOwner` MeshComp)))
  (bind _monster_actor (`/Game/project/BluePrint/Pl/BP_player.monster_Actor` _asbp_player))
  (`/Engine/EditorBlueprintResources/StandardMacros.IsValid` _monster_actor
    (:`Is Valid`
      (set `/Game/project/BluePrint/Monster/bp_monster.is_hit` false _monster_actor)
      (return false))
    (:`Is Not Valid`
      (`KismetSystemLibrary.PrintString` null "no vail"))))

(fn `Received_NotifyTick`
  (params (MeshComp :type "SkeletalMeshComponent Object Reference") (Animation :type "AnimSequenceBase Object Reference") (FrameDeltaTime :type "Float (single-precision)") (EventReference :type "AnimNotifyEventReference Structure (by ref)"))
  (returns (ReturnValue :type Boolean))
  ;[1 1 1] 코멘트
  (bind _asbp_player (cast `/Game/project/BluePrint/Pl/BP_player` (`ActorComponent.GetOwner` MeshComp)))
  (bind _battle_sward (`/Game/project/BluePrint/Pl/BP_player.battle_sward` _asbp_player))
  (bind _outhit (`KismetSystemLibrary.SphereTraceSingleForObjects` MeshComp (`SceneComponent.GetSocketLocation` _battle_sward "bone_002") (`SceneComponent.GetSocketLocation` _battle_sward "bone_200") 5.0 (`|MakeArray` "ObjectTypeQuery8" :!type "EObjectTypeQuery Enum") true))
  (bind (_bblockinghit _binitialoverlap _time _distance _location _impactpoint _normal _impactnormal _physmat _hitactor) (`GameplayStatics.BreakHitResult` _outhit))
  (if _bblockinghit
    (bind _asbp_monster (cast `/Game/project/BluePrint/Monster/bp_monster` _hitactor))
    (`GameplayStatics.ApplyDamage` _asbp_monster (`/Game/project/BluePrint/component/BPC_attackSystem.Attack_type_Damage_` (`/Game/project/BluePrint/Pl/BP_player.BPC_attackSystem` _asbp_player)) null _asbp_player)
    (return true)))