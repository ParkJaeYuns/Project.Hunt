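; AI controller for bp_monster that runs the BT_monster behavior tree and reacts to pawn sightings.
; While the monster is alive, PawnSensing sightings drive a non-looping MultiGate starting at its second output.
; That output stores the seen BP_player in the Blackboard and passes the monster to the player.
; The other output sets the battle and find Blackboard flags through a DoOnce.
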(event `self.ReceiveBeginPlay`
  (`self.RunBehaviorTree` "/Game/project/BluePrint/Monster/BT_monster.BT_monster"))

(event `self.PawnSensing.OnSeePawn`
  (params (Pawn :type "Pawn Object Reference"))
  (bind _returnvalue (`AIBlueprintHelperLibrary.GetBlackboard` self))
  (bind _asbp_monster (cast `/Game/project/BluePrint/Monster/bp_monster` (`self.K2_GetPawn`)))
  (if (not (`/Game/project/BluePrint/Monster/bp_monster.isDead` _asbp_monster))
    (`|MultiGate` false false 1
      (:`Out 0`
        ;[1 1 1] 코멘트
        (`/Engine/EditorBlueprintResources/StandardMacros.DoOnce` false
          (:`Completed`
            (`BlackboardComponent.SetValueAsBool` _returnvalue "isbattle" true)
            (`BlackboardComponent.SetValueAsBool` _returnvalue "isfind" true))))
      (:`Out 1`
        ;[1 1 1] 코멘트
        (bind _asbp_player (cast `/Game/project/BluePrint/Pl/BP_player` Pawn))
        (`BlackboardComponent.SetValueAsObject` (`AIBlueprintHelperLibrary.GetBlackboard` self) "Player" _asbp_player)
        (bind _asbp_monster_2 (cast `/Game/project/BluePrint/Monster/bp_monster` (`self.K2_GetPawn`)))
        (`/Game/project/BluePrint/Pl/BP_player.set monster actor` _asbp_player _asbp_monster_2)))))

(fn `UserConstructionScript`)