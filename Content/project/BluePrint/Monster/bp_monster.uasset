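; Monster Blueprint that handles attack setup, incoming damage, death and a timed slime state shown by a body material swap.
; A timeline turns it toward the player before calling the attack activation, and attack events set the type that selects damage.
; AnyDamage, gated by IsHit, feeds the state component, updates player sharpness and bottle charge, and briefly slows the player's montage for hit-stop.
; Death plays a montage, then ignores Pawn collision and flags the Blackboard.
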(event `self.ReceiveBeginPlay`
  (bind _asbp_player (cast `/Game/project/BluePrint/Pl/BP_player` (`GameplayStatics.GetPlayerPawn` 0))
    (:`then`
      (set `self.Player_chararcter` _asbp_player))
    (:`CastFailed`
      (`KismetSystemLibrary.PrintString` "BP_player_casting_faild"))))

(event `Focs_player`
  (params (player_location :type "Vector Structure"))
  ;[1 1 1] 코멘트
  (bind (_direction `_새_트랙_0`) (`Timeline|타임라인` :!via `PlayFromStart`)
    (:`Update`
      (`self.K2_SetActorRotation` (`KismetMathLibrary.RLerp` (`self.K2_GetActorRotation`) (`KismetMathLibrary.FindLookAtRotation` (`self.K2_GetActorLocation`) player_location) `_새_트랙_0`)))
    (:`Finished`
      (`self.activated_atttack`))))

(event `Reset_Slime`
  ;[1 1 1] 코멘트
  (`PrimitiveComponent.SetMaterialByName` (`self.Mesh`) (`self.M_Body_material_slot_name`) "/Game/project/Monster/model/MAT_EM03_body.MAT_EM03_body")
  (set `self.Activated_slime` false))

(event `activate_slime`
  ;[1 1 1] 코멘트
  (set `self.Activated_slime` true)
  (`PrimitiveComponent.SetMaterialByName` (`self.Mesh`) (`self.M_Body_material_slot_name`) "/Game/project/Monster/model/MAT_EM03_slime_mold.MAT_EM03_slime_mold")
  (`KismetSystemLibrary.K2_SetTimerDelegate` (delegate `Reset_Slime`) (`self._Slime_duration`)))

(event `ATtack_1`
  ;[1 1 1] 코멘트
  (set `self.Monster_Attack_type` "NewEnumerator2")
  (set `self.Monster_Attack_Response` "NewEnumerator2")
  (`self.Type_Damage` :!label _label))

(event `Attack_2`
  ;[1 1 1] 코멘트
  (set `self.Monster_Attack_type` "NewEnumerator3")
  (set `self.Monster_Attack_Response` "NewEnumerator2")
  (goto _label))

(event `Attack_3`
  ;[1 1 1] 코멘트
  (set `self.Monster_Attack_type` "NewEnumerator3")
  (set `self.Monster_Attack_Response` "NewEnumerator2")
  (goto _label))

(event `self.ReceiveAnyDamage`
  (params (Damage :type "Float (single-precision)") (DamageType :type "DamageType Object Reference") (InstigatedBy :type "Controller Object Reference") (DamageCauser :type "Actor Object Reference"))
  (bind _player_chararcter (`self.Player_chararcter`))
  (bind _player_chararcter_2 (`self.Player_chararcter`))
  (bind _bottle_charge_stack (`/Game/project/BluePrint/Pl/BP_player.Bottle_Charge Stack` _player_chararcter_2))
  (bind _returnvalue (`SkeletalMeshComponent.GetAnimInstance` (`Character.Mesh` _player_chararcter)))
  (bind _returnvalue_2 (`AnimInstance.GetCurrentActiveMontage` _returnvalue))
  (if (not (`self.is_hit`))
    (`/Game/project/BluePrint/Pl/BP_player.Hit_effect` _player_chararcter)
    (bind _asabp_plater (cast `/Game/project/BluePrint/Pl/ABP_plater` _returnvalue))
    (`|ExecutionSequence`
      (:`then_0`
        (bind (_is_dead _is_demaged) (`/Game/project/BluePrint/component/BPC_StateSystem.Decrease_health` (`self.BPC_StateSystem`) (make `/Game/project/BluePrint/Struct/ST_Damege_Info` Damage "NewEnumerator0" "NewEnumerator0" false false true)))
        (if _is_demaged
          (`/Game/project/BluePrint/Pl/BP_player.Decrease_Sharpness_event` _player_chararcter_2 4.0)
          (if (not (>= _bottle_charge_stack 5))
            (bind _output_get (set `/Game/project/BluePrint/Pl/BP_player.Bottle_Charge Stack` (+ _bottle_charge_stack 1) (`self.Player_chararcter`)))
            (`/Game/project/BluePrint/UI/UMG_HUD.Change_color` (`/Game/project/BluePrint/Pl/BP_player.UI` (`self.Player_chararcter`)) _output_get))
          (if _is_dead
            ;[1 1 1] 사망시
            (set `self.is_hit` true)
            (`|PlayMontage` (`self.Mesh`) "/Game/project/BluePrint/montage/monster/Dead.Dead"
              (:`OnCompleted`
                (`PrimitiveComponent.SetCollisionResponseToChannel` (`self.Mesh`) "ECC_Pawn" "ECR_Ignore")
                (`BlackboardComponent.SetValueAsBool` (`AIBlueprintHelperLibrary.GetBlackboard` self) "isDead" true)))
            (else
              (set `self.is_hit` true)))))
      (:`then_1`
        (`AnimInstance.Montage_SetPlayRate` _asabp_plater _returnvalue_2 0.01)
        (`KismetSystemLibrary.Delay` 0.1)
        (`AnimInstance.Montage_SetPlayRate` _asabp_plater _returnvalue_2 1.0)))))

(fn `Hit_effect`)

(fn `Type_Damage`
  (returns (Output_Get :type "Float (double-precision)"))
  ;[1 1 1] 코멘트
  (bind _output_get (set `self.Type_monsterDamage` (select `/Game/project/BluePrint/enum/BPE_Damage_Type` (`self.Monster_Attack_type`) :`NewEnumerator1` 150.0 :`NewEnumerator2` 200.0 :`NewEnumerator3` 250.0 :`NewEnumerator5` 150.0)))
  (return _output_get))

(fn `UserConstructionScript`)